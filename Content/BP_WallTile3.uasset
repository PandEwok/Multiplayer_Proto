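; BP_WallTile3 is a construction-script actor that fills a box sized by RoomVector with a 3D grid of instanced tile meshes.
; It divides twice RoomVector by the tile mesh's bounds to get per-axis counts, using the mesh's X size for both X and Y.
; Nested inclusive loops add one instance to Tile per cell, interior included, starting at the local origin.
; The event graph has no active logic.
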(fn `UserConstructionScript`
  (bind _returnvalue (`StaticMesh.GetBounds` (`StaticMeshComponent.StaticMesh` (`self.Tile`))))
  (bind _returnvalue_2 (* (.z (`.BoxExtent` (`KismetMathLibrary.BreakBoxSphereBounds` _returnvalue))) 2.0))
  (bind _returnvalue_3 (* (.x (`.BoxExtent` (`KismetMathLibrary.BreakBoxSphereBounds` _returnvalue))) 2.0))
  (set `self.L_Width` (`KismetMathLibrary.FTrunc` (/ (* (.x (`self.RoomVector`)) 2.0) _returnvalue_3)))
  (set `self.L_Lenght` (`KismetMathLibrary.FTrunc` (/ (* (.y (`self.RoomVector`)) 2.0) _returnvalue_3)))
  (set `self.L_Height` (`KismetMathLibrary.FTrunc` (/ (* (.z (`self.RoomVector`)) 2.0) _returnvalue_2)))
  (for _index (range (+ (`self.L_Width`) 1))
    (for _index_2 (range (+ (`self.L_Lenght`) 1))
      (for _index_3 (range (+ (`self.L_Height`) 1))
        (`InstancedStaticMeshComponent.AddInstance` (`self.Tile`) (`KismetMathLibrary.MakeTransform` (`KismetMathLibrary.MakeVector` (`KismetMathLibrary.Conv_IntToDouble` (* _index _returnvalue_3)) (`KismetMathLibrary.Conv_IntToDouble` (* _index_2 _returnvalue_3)) (`KismetMathLibrary.Conv_IntToDouble` (* _index_3 _returnvalue_2)))) false)))))