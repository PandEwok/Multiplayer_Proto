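; Grass tile actor that fills a rectangular area, sized by RoomVector, with a grid of tile mesh instances.
; The Construction Script converts RoomVector X and Y into whole tile counts on a fixed 100-unit spacing.
; Nested loops then add an instance to the Tile component at each grid point, with no active runtime logic in the Event Graph.
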(fn `UserConstructionScript`
  (set `self.L_Width` (`KismetMathLibrary.FTrunc` (/ (.x (`self.RoomVector`)) 100.0)))
  (set `self.L_Lenght` (`KismetMathLibrary.FTrunc` (/ (.y (`self.RoomVector`)) 100.0)))
  (for _index (range (+ (`self.L_Width`) 1))
    (for _index_2 (range (+ (`self.L_Lenght`) 1))
      (`InstancedStaticMeshComponent.AddInstance` (`self.Tile`) (`KismetMathLibrary.MakeTransform` (`KismetMathLibrary.MakeVector` (`KismetMathLibrary.Conv_IntToDouble` (* _index 100)) (`KismetMathLibrary.Conv_IntToDouble` (* _index_2 100)))) false))))